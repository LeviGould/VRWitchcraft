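; Hand component that detects finger curls on a tracked hand to recognise a pointing gesture.
; Each tick it measures the distance from the index, ring, middle and pinky tip bones to named sockets, treating a finger as down within a threshold.
; Middle, ring and pinky down with index up sets Pointing.
; Curling the index from that pose fires OnPoint and clears Pointing, acting like a trigger pull.
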(event EventBeginPlay)

(event EventTick
  (params (DeltaSeconds :type Float%20%28single-precision%29))
  (Utilities|FlowControl|Sequence
    (:then_0
      (bind _return (CallFunction|IsFingerDown? (Variables|Default|GetIndexTipBone) (Variables|Default|GetIndexTipBone)))
      (if _return
        (if (not (Variables|Default|GetbIndexDown))
          (Variables|Default|SetbIndexDown (not (Variables|Default|GetbIndexDown)) :!label _label))
        (elif (Variables|Default|GetbIndexDown)
          (goto _label))))
    (:then_1
      (bind _return_2 (CallFunction|IsFingerDown? (Variables|Default|GetRingTipBone) (Variables|Default|GetRingFingerSocket)))
      (if _return_2
        (if (not (Variables|Default|GetbRingDown))
          (Variables|Default|SetbRingDown (not (Variables|Default|GetbRingDown)) :!label _label_2))
        (elif (Variables|Default|GetbRingDown)
          (goto _label_2))))
    (:then_2
      (bind _return_3 (CallFunction|IsFingerDown? (Variables|Default|GetMiddleTipBone) (Variables|Default|GetMiddleFingerSocket)))
      (if _return_3
        (if (not (Variables|Default|GetbMiddleDown))
          (Variables|Default|SetbMiddleDown (not (Variables|Default|GetbMiddleDown)) :!label _label_3))
        (elif (Variables|Default|GetbMiddleDown)
          (goto _label_3))))
    (:then_3
      (bind _return_4 (CallFunction|IsFingerDown? (Variables|Default|GetPinkyTipBone) (Variables|Default|GetPinkyFingerSocket)))
      (if _return_4
        (if (not (Variables|Default|GetbPinkyDown))
          (Variables|Default|SetbPinkyDown (not (Variables|Default|GetbPinkyDown)) :!label _label_4))
        (elif (Variables|Default|GetbPinkyDown)
          (goto _label_4))))
    (:then_4
      (if (Math|Boolean|ANDBoolean (Variables|Default|GetbPinkyDown) (Variables|Default|GetbMiddleDown) (Variables|Default|GetbRingDown) (not (Variables|Default|GetbIndexDown)))
        (if (not (Variables|Default|GetbPointing))
          (Variables|Default|SetbPointing true))
        (elif (Math|Boolean|ANDBoolean (Variables|Default|GetbPinkyDown) (Variables|Default|GetbMiddleDown) (Variables|Default|GetbRingDown) (Variables|Default|GetbIndexDown))
          (if (Variables|Default|GetbPointing)
            (Default|CallOnPoint))
          (Variables|Default|SetbPointing false)
          (else
            (Variables|Default|SetbPointing false)))))))

(fn IsFingerDown?
  (params (BoneName :type Name) (SocketName :type Name))
  (bind _returnvalue (Class|PoseableMeshComponent|GetBoneLocationbyName BoneName "WorldSpace"))
  (if true
    (return (< (Math|Float|Absolute(Float) (Math|Vector|VectorLength (- _returnvalue (Transformation|GetSocketLocation SocketName)))) (Variables|Default|GetThreshold)))))